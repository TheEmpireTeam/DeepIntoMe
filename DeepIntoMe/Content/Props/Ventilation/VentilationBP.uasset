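; Procedural ventilation duct prop that builds itself along a spline path in the construction script.
; Each spline segment snaps to its dominant world axis and is filled with fixed-length duct meshes, with fans added at random by a probability.
; An air intake mesh is placed at each segment's end point.
; Ducts and intakes get dynamic metal materials tinted by a color variable.
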(event EventBeginPlay)

(event EventActorBeginOverlap
  (params (OtherActor :type Actor%20Object%20Reference)))

(fn ConstructionScript
  (CallFunction|GetPoint (Variables|Default|Getpath)))

(fn DrawBetweenPoints
  (params (startPoint :type Vector) (endPoint :type Vector))
  (Variables|Default|SetPoint startPoint)
  (bind (_stepx _stepy _stepz _rotation _count) (CallFunction|ResolveDirection startPoint endPoint))
  (Variables|Default|SetstepX _stepx)
  (Variables|Default|SetstepY _stepy)
  (Variables|Default|SetstepZ _stepz)
  (Variables|Default|Setrotar _rotation)
  (bind _output_get (Variables|Default|Setcount _count))
  (for _index (range 1 _output_get)
    (CallFunction|Draw)))

(fn Draw
  (bind _returnvalue (AddComponent|AddStaticMeshComponent false (Math|Transform|MakeTransform (- (Variables|Default|GetPoint) (Transformation|GetWorldLocation (Variables|Default|GetDefaultSceneRoot))) (Variables|Default|Getrotar))))
  (Components|StaticMesh|SetStaticMesh _returnvalue "/Game/Props/Ventilation/Ventilation_ventilation.Ventilation_ventilation")
  (bind _returnvalue_2 (Rendering|Material|CreateDynamicMaterialInstance "/Game/Props/Ventilation/Ventilation_Metall.Ventilation_Metall" :!class /Script/Engine.KismetMaterialLibrary))
  (Rendering|Material|SetVectorParameterValue _returnvalue_2 "Color" (Variables|Default|GetColor) :!class /Script/Engine.MaterialInstanceDynamic)
  (Rendering|Material|SetMaterial _returnvalue 0 _returnvalue_2)
  (if (< (Math|Random|RandomInteger 100) (Variables|Default|Getprobability))
    (bind _returnvalue_3 (AddComponent|AddStaticMeshComponent false (Math|Transform|MakeTransform (- (Variables|Default|GetPoint) (Transformation|GetWorldLocation (Variables|Default|GetDefaultSceneRoot))) (Variables|Default|Getrotar))))
    (Components|StaticMesh|SetStaticMesh _returnvalue_3 "/Game/Props/Ventilation/Ventilation_Fan.Ventilation_Fan"))
  (Variables|Default|SetPoint (Math|Vector|MakeVector (+ (Variables|Default|GetstepX) (.X (Math|Vector|BreakVector (Variables|Default|GetPoint)))) (+ (.Y (Math|Vector|BreakVector (Variables|Default|GetPoint))) (Variables|Default|GetstepY)) (+ (.Z (Math|Vector|BreakVector (Variables|Default|GetPoint))) (Variables|Default|GetstepZ))))
  (return))

(fn GetPoint
  (params (Spline :type Spline%20Component%20Object%20Reference))
  (for _index (range 0 (- (Spline|GetNumberOfSplinePoints Spline) 2))
    (CallFunction|DrawBetweenPoints (Spline|GetLocationatSplinePoint Spline _index "World") (Spline|GetLocationatSplinePoint Spline (+ _index 1) "World"))
    (CallFunction|DrawAirIntake (Spline|GetLocationatSplinePoint Spline (+ _index 1) "World"))))

(fn DrawAirIntake
  (params (Location :type Vector))
  (bind _returnvalue (AddComponent|AddStaticMeshComponent false (Math|Conversions|ToTransform(Vector) (- Location (Transformation|GetWorldLocation (Variables|Default|GetDefaultSceneRoot))))))
  (Components|StaticMesh|SetStaticMesh _returnvalue "/Game/Props/Ventilation/Ventilation_2.Ventilation_2")
  (bind _returnvalue_2 (Rendering|Material|CreateDynamicMaterialInstance "/Game/Props/Ventilation/Ventilation_Metall.Ventilation_Metall" :!class /Script/Engine.KismetMaterialLibrary))
  (Rendering|Material|SetVectorParameterValue _returnvalue_2 "Color" (Variables|Default|GetColor) :!class /Script/Engine.MaterialInstanceDynamic)
  (Rendering|Material|SetMaterial _returnvalue 0 _returnvalue_2))

(fn ResolveDirection
  (params (startPosition :type Vector) (endPosition :type Vector))
  (bind (_x _y _z) (Math|Vector|BreakVector startPosition))
  (bind (_x_2 _y_2 _z_2) (Math|Vector|BreakVector endPosition))
  (bind _output_get (LocalVariables|SetxDistance (- _x _x_2)))
  (bind _output_get_2 (LocalVariables|SetyDistance (- _y _y_2)))
  (bind _output_get_3 (LocalVariables|SetzDistance (- _z _z_2)))
  (switch int (.IndexOfMaxValue (Math|Float|MaxOfFloatArray (Utilities|Array|MakeArray (Math|Float|Absolute(Float) _output_get) (Math|Float|Absolute(Float) _output_get_2) (Math|Float|Absolute(Float) _output_get_3))))
    (:Default
      (LocalVariables|SetyStep 0.0 :!label _label)
      (LocalVariables|SetzStep 0.0)
      (LocalVariables|Setrot "0, 0, 0")
      (if (< (LocalVariables|GetxDistance) 0.0)
        (LocalVariables|SetxStep (Variables|Default|Getventilation_length))
        (else
          (LocalVariables|SetxStep (* (Variables|Default|Getventilation_length) -1.0))))
      (LocalVariables|Setcol (Math|Float|Truncate (Math|Float|Absolute(Float) (/ (LocalVariables|GetxDistance) (Variables|Default|Getventilation_length))))))
    (:0
      (goto _label))
    (:1
      (LocalVariables|SetxStep 0.0)
      (LocalVariables|SetzStep 0.0)
      (LocalVariables|Setrot "0.000000,90.000000, 0")
      (if (< (LocalVariables|GetyDistance) 0.0)
        (LocalVariables|SetyStep (Variables|Default|Getventilation_length))
        (else
          (LocalVariables|SetyStep (* (Variables|Default|Getventilation_length) -1.0))))
      (LocalVariables|Setcol (Math|Float|Truncate (Math|Float|Absolute(Float) (/ (LocalVariables|GetyDistance) (Variables|Default|Getventilation_length))))))
    (:2
      (LocalVariables|SetxStep 0.0)
      (LocalVariables|SetyStep 0.0)
      (LocalVariables|Setrot "90.000000,0.000000, 0")
      (if (< (LocalVariables|GetzDistance) 0.0)
        (LocalVariables|SetzStep (Variables|Default|Getventilation_length))
        (else
          (LocalVariables|SetzStep (* (Variables|Default|Getventilation_length) -1.0))))
      (LocalVariables|Setcol (Math|Float|Truncate (Math|Float|Absolute(Float) (/ (LocalVariables|GetzDistance) (Variables|Default|Getventilation_length)))))))
  (return (LocalVariables|GetxStep) (LocalVariables|GetyStep) (LocalVariables|GetzStep) (LocalVariables|Getrot) (LocalVariables|Getcol)))