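; Industrial light prop that pairs a mesh with a spot light, configurable by color, intensity, radius and cone angles.
; The construction script creates a dynamic material for the emissive glow and applies matching settings to the spot light.
; TurnOn, TurnOff and Switch change the on state and rerun both setup functions, zeroing emissive level and light intensity when off.
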(event EventBeginPlay)

(event EventActorBeginOverlap
  (params (OtherActor :type Actor%20Object%20Reference)))

(event EventTick
  (params (DeltaSeconds :type Float%20%28single-precision%29)))

(fn ConstructionScript
  (CallFunction|SetMaterial)
  (CallFunction|SetLight))

(fn SetMaterial
  (bind _returnvalue (Rendering|Material|CreateDynamicMaterialInstance (Variables|Default|GetIndustrial_light_mesh) 0 "/Game/Props/Lighters/Industrial_light/industrial_lighter_Inst.industrial_lighter_Inst" :!class /Script/Engine.PrimitiveComponent))
  (Rendering|Material|SetVectorParameterValue _returnvalue "Emissive color" (Variables|Default|GetColor) :!class /Script/Engine.MaterialInstanceDynamic)
  (if (Variables|Default|GetTurn%20On)
    (Rendering|Material|SetScalarParameterValue _returnvalue "Emissive_level" (Variables|Default|GetIntensity) :!class /Script/Engine.MaterialInstanceDynamic)
    (else
      (Rendering|Material|SetScalarParameterValue _returnvalue "Emissive_level" 0.0 :!class /Script/Engine.MaterialInstanceDynamic)))
  (Rendering|Material|SetMaterial (Variables|Default|GetIndustrial_light_mesh) 0 _returnvalue)
  (return))

(fn SetLight
  (bind _spotlight (Variables|Default|GetSpotLight))
  (Rendering|Components|Light|SetLightColor _spotlight (Variables|Default|GetColor) true)
  (Rendering|Lighting|SetAttenuationRadius _spotlight (Variables|Default|GetRadius))
  (Rendering|Lighting|SetOuterConeAngle _spotlight (Variables|Default|GetOuterAngle))
  (Rendering|Lighting|SetInnerConeAngle _spotlight (Variables|Default|GetInnerAngle))
  (if (Variables|Default|GetTurn%20On)
    (Rendering|Components|Light|SetIntensity _spotlight (Variables|Default|GetIntensity))
    (else
      (Rendering|Components|Light|SetIntensity _spotlight 0.0)))
  (return))

(fn Turnon
  (if (Variables|Default|GetTurn%20On)
    _
    (else
      (Variables|Default|SetTurn%20On true)
      (CallFunction|SetMaterial)
      (CallFunction|SetLight)))
  (return))

(fn TurnOff
  (if (Variables|Default|GetTurn%20On)
    (Variables|Default|SetTurn%20On false)
    (CallFunction|SetMaterial)
    (CallFunction|SetLight))
  (return))

(fn Switch
  (if (Variables|Default|GetTurn%20On)
    (CallFunction|TurnOff)
    (else
      (CallFunction|Turnon)))
  (return))