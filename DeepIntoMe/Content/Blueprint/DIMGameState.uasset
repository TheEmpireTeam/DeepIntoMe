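; DIMGameState is a game state Blueprint that maintains PlayersList, a list of the DIMPlayerState actors in the game.
; Every Tick it gets all DIMPlayerState actors and searches PlayersList for each, resetting a PlayerFound flag per actor.
; The add check runs after the outer loop completes, so only the last actor iterated can be appended when missing from the list.
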(event EventBeginPlay)

(event EventTick
  (params (DeltaSeconds :type Float%20%28single-precision%29))
  (bind _outactors (Actor|GetAllActorsOfClass "/Game/Blueprint/DIMPlayerState.DIMPlayerState_C"))
  (for _array_element _outactors
    (Variables|Default|SetPlayer%20Found false)
    (for _array_element_2 (Variables|Default|GetPlayersList)
      (if (== _array_element_2 _array_element)
        (Variables|Default|SetPlayer%20Found true))))
  (if (not (Variables|Default|GetPlayer%20Found))
    (bind _asdimplayer_state (Utilities|Casting|CastToDIMPlayerState _array_element))
    (Utilities|Array|Add (Variables|Default|GetPlayersList) _asdimplayer_state)))

(fn ConstructionScript)