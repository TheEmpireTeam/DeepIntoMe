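; Player character Blueprint that detects interactive panels in view and tints the body by team.
; Every Tick it line-traces forward from the camera against WorldStatic objects, setting a hit InteractivePanel as the focused interactable and clearing focus otherwise.
; UpdateTeamColor maps the team (Spectator, Earth, Bailosh or Aliens) to a color and applies it through a new dynamic material instance of the mannequin body material.
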(event EventBeginPlay)

(event EventActorBeginOverlap
  (params (OtherActor :type Actor%20Object%20Reference)))

(event EventTick
  (params (DeltaSeconds :type Float%20%28single-precision%29))
  (bind _camera (Variables|Default|GetCamera))
  (bind _returnvalue (Transformation|GetWorldLocation _camera))
  (bind (_outhit _returnvalue_2) (Collision|LineTraceForObjects _returnvalue (+ _returnvalue (* (Math|Vector|GetForwardVector (Transformation|GetWorldRotation _camera)) (Variables|Default|GetTrace%20Radius))) (Utilities|Array|MakeArray "ObjectTypeQuery1") false 0 "None"))
  (if _returnvalue_2
    (bind _asinteractive_panel (Utilities|Casting|CastToInteractivePanel (.HitActor (Collision|BreakHitResult _outhit)))
      (:then
        (Class|MainCharacter|SetFocusedInteractableActor _asinteractive_panel))
      (:CastFailed
        (Class|MainCharacter|SetFocusedInteractableActor :!label _label)))
    (else
      (goto _label))))

(event EventUpdateTeamColor
  (params (Team :type EMultiplayerTeam%20Enum :default "Spectator"))
  (switch Utilities|FlowControl|Switch|SwitchonEMultiplayerTeam Team
    (:Spectator
      (Variables|Default|SetColor "(R=1.000000,G=1.000000,B=1.000000,A=1.000000)"))
    (:Earth
      (Variables|Default|SetColor "(R=1.000000,G=0.501867,B=0.167414,A=1.000000)"))
    (:Bailosh
      (Variables|Default|SetColor "(R=0.193402,G=0.422066,B=1.000000,A=1.000000)"))
    (:Aliens
      (Variables|Default|SetColor "(R=0.193402,G=0.422066,B=0.000000,A=1.000000)")))
  (bind _returnvalue (Rendering|Material|CreateDynamicMaterialInstance (Variables|Character|GetMesh) 0 "/Game/AnimStarterPack/UE4_Mannequin/Materials/M_UE4Man_Body.M_UE4Man_Body" :!class /Script/Engine.PrimitiveComponent))
  (Rendering|Material|SetVectorParameterValue _returnvalue "BodyColor" (Variables|Default|GetColor) :!class /Script/Engine.MaterialInstanceDynamic)
  (Rendering|Material|SetMaterial (Variables|Character|GetMesh) 0 _returnvalue))

(fn ConstructionScript)